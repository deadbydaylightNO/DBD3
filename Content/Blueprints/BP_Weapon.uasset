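; Weapon actor that counts hits on human AI characters and hides its mesh during the first-person player's special attack.
; Tick polls the player's special-attack flag to toggle mesh visibility.
; Overlaps increment a counter on the weapon, shared across targets: the first prints an injured state and briefly disables capsule collision as a re-hit cooldown.
; The next prints a stunned state and resets the counter; both states are only debug prints here.
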(event `self.ReceiveBeginPlay`)

(event `self.ReceiveTick`
  (params (DeltaSeconds :type "Float (single-precision)"))
  (bind _asbp_first_person_character (cast `/Game/FirstPerson/Blueprints/BP_FirstPersonCharacter` (`GameplayStatics.GetPlayerPawn` 0)))
  (if (`/Game/FirstPerson/Blueprints/BP_FirstPersonCharacter.IsSpecialAttack` _asbp_first_person_character)
    (`SceneComponent.SetVisibility` (`self.StaticMesh`) false false)
    (else
      (`SceneComponent.SetVisibility` (`self.StaticMesh`) true false))))

(event `self.ReceiveActorBeginOverlap`
  (params (OtherActor :type "Actor Object Reference"))
  (bind _deathcount (`self.DeathCount`))
  (cast `/Game/OJS/BP_humanAiCharacter` OtherActor)
  (bind _result (`/Engine/EditorBlueprintResources/StandardMacros.IncrementInt` _deathcount)
    (:`  `
      (`KismetSystemLibrary.PrintString` (`KismetStringLibrary.Conv_IntToString` _result))
      (if (== _deathcount 1)
        (`KismetSystemLibrary.PrintString` "부상상태 / BP_Weapon")
        (`PrimitiveComponent.SetCollisionEnabled` (`self.Capsule`) "NoCollision")
        (`KismetSystemLibrary.Delay` 0.8)
        (`PrimitiveComponent.SetCollisionEnabled` (`self.Capsule`) "QueryOnly")
        (else
          (`KismetSystemLibrary.PrintString` "기절상태 / BP_Weapon")
          (set `self.DeathCount` 0))))))

(fn `UserConstructionScript`)