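; BP_SpecialATK is a special-attack projectile, apparently the killer's, that knocks out the four generators.
; Tick moves it along its forward vector by Speed and delta time, without sweeping.
; Overlapping gen1–gen4 turns that generator's light red, calls its Off function and Startengine on the matching BP_Generator_Single_TEST actors, and prints a Korean shutdown message.
; A Landscape hit destroys it and leaves a short-lived killer decal.
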(event `self.ReceiveActorBeginOverlap`
  (params (OtherActor :type "Actor Object Reference"))
  (`|ExecutionSequence`
    (:`then_0`
      (bind _asgen_1 (cast `/Game/OJS/engine/gen1` OtherActor))
      (`|ExecutionSequence`
        (:`then_0`
          (`SceneComponent.SetVisibility` (`/Game/OJS/engine/gen1.PointLightRED` _asgen_1) true false))
        (:`then_1`
          (`SceneComponent.SetVisibility` (`/Game/OJS/engine/gen1.PointLightGreen` _asgen_1) false false))
        (:`then_2`
          (bind _outactors (`GameplayStatics.GetAllActorsOfClass` "/Game/OJS/engine/BP_Generator_Single_TEST1.BP_Generator_Single_TEST1_C"))
          (`/Game/OJS/engine/BP_Generator_Single_TEST1.startengine1` _outactors)
          (`/Game/OJS/engine/gen1.Gen1Off` _asgen_1)
          (`KismetSystemLibrary.PrintString` "첫번째 엔진이 꺼졌습니다." true true (struct :`R` 1.0 :`B` 0.019289 :`A` 1.0) 5.0))))
    (:`then_1`
      (bind _asgen_2 (cast `/Game/OJS/engine/gen2` OtherActor))
      (`|ExecutionSequence`
        (:`then_0`
          (`SceneComponent.SetVisibility` (`/Game/OJS/engine/gen2.PointLightGreen` _asgen_2) false false))
        (:`then_1`
          (`SceneComponent.SetVisibility` (`/Game/OJS/engine/gen2.PointLightRED` _asgen_2) true false))
        (:`then_2`
          (bind _outactors_2 (`GameplayStatics.GetAllActorsOfClass` "/Game/OJS/engine/BP_Generator_Single_TEST2.BP_Generator_Single_TEST2_C"))
          (`/Game/OJS/engine/BP_Generator_Single_TEST2.startengine2` _outactors_2)
          (`/Game/OJS/engine/gen2.Gen2OFF` _asgen_2)
          (`KismetSystemLibrary.PrintString` "두번째 엔진이 꺼졌습니다." true true (struct :`R` 1.0 :`B` 0.019289 :`A` 1.0) 5.0))))
    (:`then_2`
      (bind _asgen_3 (cast `/Game/OJS/engine/gen3` OtherActor))
      (`|ExecutionSequence`
        (:`then_0`
          (`SceneComponent.SetVisibility` (`/Game/OJS/engine/gen3.PointLightGreen` _asgen_3) false false))
        (:`then_1`
          (`SceneComponent.SetVisibility` (`/Game/OJS/engine/gen3.PointLightRED` _asgen_3) true false))
        (:`then_2`
          (bind _outactors_3 (`GameplayStatics.GetAllActorsOfClass` "/Game/OJS/engine/BP_Generator_Single_TEST3.BP_Generator_Single_TEST3_C"))
          (`/Game/OJS/engine/BP_Generator_Single_TEST3.startengine3` _outactors_3)
          (`/Game/OJS/engine/gen3.gen3Off` _asgen_3)
          (`KismetSystemLibrary.PrintString` "세번째 엔진이 꺼졌습니다." true true (struct :`R` 1.0 :`B` 0.019289 :`A` 1.0) 5.0))))
    (:`then_3`
      (bind _asgen_4 (cast `/Game/OJS/engine/gen4` OtherActor))
      (`|ExecutionSequence`
        (:`then_0`
          (`SceneComponent.SetVisibility` (`/Game/OJS/engine/gen4.PointLightGreen` _asgen_4) false false))
        (:`then_1`
          (`SceneComponent.SetVisibility` (`/Game/OJS/engine/gen4.PointLightRED` _asgen_4) true false))
        (:`then_2`
          (bind _outactors_4 (`GameplayStatics.GetAllActorsOfClass` "/Game/OJS/engine/BP_Generator_Single_TEST4.BP_Generator_Single_TEST4_C"))
          (`/Game/OJS/engine/BP_Generator_Single_TEST4.startengine4` _outactors_4)
          (`/Game/OJS/engine/gen4.gen4Off` _asgen_4)
          (`KismetSystemLibrary.PrintString` "네번째 엔진이 꺼졌습니다." true true (struct :`R` 1.0 :`B` 0.019289 :`A` 1.0) 5.0))))))

(event `self.ReceiveHit`
  (params (MyComp :type "PrimitiveComponent Object Reference") (Other :type "Actor Object Reference") (OtherComp :type "PrimitiveComponent Object Reference") (bSelfMoved :type Boolean) (HitLocation :type "Vector Structure") (HitNormal :type "Vector Structure") (NormalImpulse :type "Vector Structure") (Hit :type "HitResult Structure (by ref)"))
  (cast `Landscape` Other)
  (`self.K2_DestroyActor`)
  (`GameplayStatics.SpawnDecalAttached` "/Game/Killer/KillerDecalTexture/Mat_KillerDecal.Mat_KillerDecal" (55.0 55.0 55.0) OtherComp "None" HitLocation (`KismetMathLibrary.Conv_VectorToRotator` HitNormal) "KeepWorldPosition" 5.0))

(event `self.ReceiveTick`
  (params (DeltaSeconds :type "Float (single-precision)"))
  (`self.Translate` (`self.GetActorForwardVector`) (`self.Speed`)))

(fn `Translate`
  (params (Direction :type "Vector Structure") (Speed :type "Float (double-precision)"))
  ;[1 1 1] P = P0 + velocity(dir * speed)*deltaSecond
  (`self.K2_SetActorLocation` (+ (`self.K2_GetActorLocation`) (* Direction Speed (`GameplayStatics.GetWorldDeltaSeconds`)))))

(fn `UserConstructionScript`)