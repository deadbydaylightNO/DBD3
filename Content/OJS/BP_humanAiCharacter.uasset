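; AI human character that continually flees from the first-person player.
; From BeginPlay, a self-restarting AIMoveTo loop picks random reachable points around a spot directly away from the player, retrying on success or failure.
; Overlaps with BP_SpecialATK increment a counter that, at a threshold, only prints an infection-state message.
; Left footsteps spawn temporary decals at the toe socket; chase-player logic is left unconnected.
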(event `self.ReceiveActorBeginOverlap`
  (params (OtherActor :type "Actor Object Reference"))
  (cast `/Game/Blueprints/BP_SpecialATK` OtherActor)
  (bind _result (`/Engine/EditorBlueprintResources/StandardMacros.IncrementInt` (`self.overlapATK`))
    (:`  `
      (bind _output_get (set `self.overlapATK` _result))
      (if (>= _output_get 10)
        (`KismetSystemLibrary.PrintString` "감염상태 / BP_humanAiCharacter")))))

(event `runPlayer`)

(event `self.ReceiveBeginPlay`
  (bind _asbp_first_person_character (cast `/Game/FirstPerson/Blueprints/BP_FirstPersonCharacter` (`GameplayStatics.GetPlayerCharacter` 0)))
  (set `self.CharREF` _asbp_first_person_character)
  (`self.runAway`))

(event `runAway`
  (bind _returnvalue (`self.K2_GetActorLocation`))
  (`|AIMoveTo` self (`NavigationSystemV1.K2_GetRandomReachablePointInRadius` (`KismetMathLibrary.MakeVector` (.x (+ _returnvalue (* (`KismetMathLibrary.GetForwardVector` (`KismetMathLibrary.FindLookAtRotation` _returnvalue (`self.K2_GetActorLocation` (`self.CharREF`)))) -500.0))) (.y (+ _returnvalue (* (`KismetMathLibrary.GetForwardVector` (`KismetMathLibrary.FindLookAtRotation` _returnvalue (`self.K2_GetActorLocation` (`self.CharREF`)))) -500.0))) (.z _returnvalue)) 500.0 null null) null
    (:`OnSuccess`
      _)
    (:`OnFail`
      _))
  (`self.runAway`))

(event `FootStep`
  (params (IsLeftFoot :type Boolean))
  (if IsLeftFoot
    (`GameplayStatics.SpawnDecalAtLocation` "/Game/OJS/decal/M_Decal.M_Decal" (100.0 100.0 100.0) (`SceneComponent.GetSocketLocation` (`self.Mesh`) "LeftToe_EndSocket") (struct) 10.0)))

(fn `UserConstructionScript`)