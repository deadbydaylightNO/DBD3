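; BP_brian is the AI character Brian, driven by state flags for sight, running, repairing, infection and hit boosts.
; PawnSensing flags a seen first-person player in the Blackboard, while BrainRepair toggles repair flags around a timed delay.
; From the tenth BP_SpecialATK overlap, infection temporarily slows him and adds an aura overlay.
; Tick applies WalkSpeedB to movement, including a short hit boost, and left footsteps spawn temporary decals.
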(event `self.ReceiveActorBeginOverlap`
  (params (OtherActor :type "Actor Object Reference"))
  (bind _mesh (`self.Mesh`))
  (cast `/Game/Blueprints/BP_SpecialATK` OtherActor)
  (bind _result (`/Engine/EditorBlueprintResources/StandardMacros.IncrementInt` (`self.Overlap ATK`))
    (:`  `
      (bind _output_get (set `self.Overlap ATK` _result))
      (if (>= _output_get 10)
        (`KismetSystemLibrary.PrintString` "감염상태 / brian")
        (`|ExecutionSequence`
          (:`then_0`
            (set `self.WalkSpeed_B` 280.0)
            (set `self.poisonChkB` true)
            (`KismetSystemLibrary.Delay` 3.0)
            (set `self.poisonChkB` false)
            (set `self.WalkSpeed_B` 380.0))
          (:`then_1`
            (`MeshComponent.SetOverlayMaterial` _mesh "/Game/OJS/aura/Aura1.Aura1")
            (`KismetSystemLibrary.Delay` 3.0)
            (`MeshComponent.SetOverlayMaterial` _mesh null)))))))

(event `self.ReceiveTick`
  (params (DeltaSeconds :type "Float (single-precision)"))
  (`|ExecutionSequence`
    (:`then_0`
      (if (`self.HitBoostB`)
        (set `self.WalkSpeed_B` 1500.0)
        (`KismetSystemLibrary.Delay` 2.0)
        (set `self.HitBoostB` false)
        (set `self.WalkSpeed_B` 450.0)))
    (:`then_1`
      (set `CharacterMovementComponent.MaxWalkSpeed` (`self.WalkSpeed_B`) (`self.CharacterMovement`)))))

(event `BrianRun`
  (if (`self.poisonChkB`)
    (set `self.WalkSpeed_B` 280.0)
    (else
      (set `self.WalkSpeed_B` 450.0))))

(event `self.PawnSensing.OnSeePawn`
  (params (Pawn :type "Pawn Object Reference"))
  (cast `/Game/FirstPerson/Blueprints/BP_FirstPersonCharacter` Pawn)
  (`BlackboardComponent.SetValueAsBool` (`AIBlueprintHelperLibrary.GetBlackboard` (`AIBlueprintHelperLibrary.GetAIController` self)) "hadSeenPlayerByBrain" true)
  (set `self.RunSwitch_B` true)
  (set `self.SeeCheck` true))

(event `BrainRepair`
  (set `self.RepairService_B` true)
  (`KismetSystemLibrary.Delay` 30.0)
  (`|ExecutionSequence`
    (:`then_0`
      (set `self.RepairService_B` false))
    (:`then_1`
      (set `self.reapir2B` true))))

(event `FootStepBrian`
  (params (isLeftFoot :type Boolean))
  (if isLeftFoot
    (`GameplayStatics.SpawnDecalAtLocation` "/Game/OJS/decal/M_Decal3.M_Decal3" (100.0 100.0 100.0) (`SceneComponent.GetSocketLocation` (`self.Mesh`) "LeftToe_EndSocket") (struct :`Pitch` 90.0 :`Roll` 90.0) 5.0)))

(fn `UserConstructionScript`)