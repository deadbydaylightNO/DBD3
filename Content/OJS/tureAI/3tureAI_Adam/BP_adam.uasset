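; BP_adam is the Adam AI character, which hunts the player and can be infected by special attacks.
; From the tenth BP_SpecialATK overlap onward, each hit briefly slows it and applies an aura overlay.
; Pawn sensing flags player sightings on the Blackboard, while run and infection logic set the walk speed that Tick applies to movement.
; Other events hold a timed repair flag and spawn footprint decals.
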(event `self.ReceiveActorBeginOverlap`
  (params (OtherActor :type "Actor Object Reference"))
  (bind _mesh (`self.Mesh`))
  (cast `/Game/Blueprints/BP_SpecialATK` OtherActor)
  (bind _result (`/Engine/EditorBlueprintResources/StandardMacros.IncrementInt` (`self.Overlap ATK`))
    (:`  `
      (bind _output_get (set `self.Overlap ATK` _result))
      (if (>= _output_get 10)
        (`KismetSystemLibrary.PrintString` "감염상태 / Adam")
        (`|ExecutionSequence`
          (:`then_0`
            (set `self.WalkSpeed_A` 280.0)
            (set `self.poisonChkA` true)
            (`KismetSystemLibrary.Delay` 3.0)
            (set `self.poisonChkA` false)
            (set `self.WalkSpeed_A` 380.0))
          (:`then_1`
            (`MeshComponent.SetOverlayMaterial` _mesh "/Game/OJS/aura/Aura1.Aura1")
            (`KismetSystemLibrary.Delay` 3.0)
            (`MeshComponent.SetOverlayMaterial` _mesh null)))))))

(event `self.ReceiveTick`
  (params (DeltaSeconds :type "Float (single-precision)"))
  (set `CharacterMovementComponent.MaxWalkSpeed` (`self.WalkSpeed_A`) (`self.CharacterMovement`)))

(event `AdamRun`
  (if (`self.poisonChkA`)
    (set `self.WalkSpeed_A` 280.0)
    (else
      (set `self.WalkSpeed_A` 450.0))))

(event `self.PawnSensing.OnSeePawn`
  (params (Pawn :type "Pawn Object Reference"))
  (cast `/Game/FirstPerson/Blueprints/BP_FirstPersonCharacter` Pawn)
  (`BlackboardComponent.SetValueAsBool` (`AIBlueprintHelperLibrary.GetBlackboard` (`AIBlueprintHelperLibrary.GetAIController` self)) "hadSeenPlayerByAdam" true)
  (set `self.RunSwitch_A` true)
  (set `self.SeeCheck_A` true))

(event `AdamRepair`
  (set `self.RepairService_A` true)
  (`KismetSystemLibrary.Delay` 13.0)
  (set `self.RepairService_A` false))

(event `FootStepAdam`
  (params (IsLeftFoot :type Boolean))
  (if IsLeftFoot
    (`GameplayStatics.SpawnDecalAtLocation` "/Game/OJS/decal/M_Decal2.M_Decal2" (100.0 100.0 100.0) (`SceneComponent.GetSocketLocation` (`self.Mesh`) "RightToe_EndSocket") (struct :`Pitch` 90.0 :`Roll` 90.0) 5.0)))

(fn `UserConstructionScript`)