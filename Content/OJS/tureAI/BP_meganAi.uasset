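; BP_meganAi is an AI character that reacts to seeing the first-person player and leaves footprint decals.
; PawnSensing sets the blackboard key hadSeenPlayer2 and a run-switch flag when it spots BP_FirstPersonCharacter.
; Tick copies WalkSpeed to movement speed, which the RUN event raises, while repairSerivce holds a repair flag on for a timed delay.
; FootStep2 spawns a short-lived decal at the right toe socket, only when IsLeftFoot is true.
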(event `self.ReceiveBeginPlay`)

(event `self.ReceiveTick`
  (params (DeltaSeconds :type "Float (single-precision)"))
  (set `CharacterMovementComponent.MaxWalkSpeed` (`self.WalkSpeed`) (`self.CharacterMovement`)))

(event `RUN`
  (set `self.WalkSpeed` 600.0))

(event `self.PawnSensing.OnSeePawn`
  (params (Pawn :type "Pawn Object Reference"))
  (cast `/Game/FirstPerson/Blueprints/BP_FirstPersonCharacter` Pawn)
  (`BlackboardComponent.SetValueAsBool` (`AIBlueprintHelperLibrary.GetBlackboard` (`AIBlueprintHelperLibrary.GetAIController` self)) "hadSeenPlayer2" true)
  (set `self.RunSwitchM` true))

(event `repairSerivce`
  (set `self.RepairServiceM` true)
  (`KismetSystemLibrary.Delay` 13.0)
  (set `self.RepairServiceM` false))

(event `FootStep2`
  (params (IsLeftFoot :type Boolean))
  (if IsLeftFoot
    (`GameplayStatics.SpawnDecalAtLocation` "/Game/OJS/decal/M_Decal2.M_Decal2" (100.0 100.0 100.0) (`SceneComponent.GetSocketLocation` (`self.Mesh`) "RightToe_EndSocket") (struct :`Pitch` 90.0 :`Roll` 90.0) 5.0)))

(fn `UserConstructionScript`)